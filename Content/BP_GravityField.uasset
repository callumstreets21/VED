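; Gravity field actor that pulls overlapping third-person characters toward its center by setting their movement component's gravity direction every Tick.
; The construction script generates a procedural sphere mesh with a material, while a box mesh alternative with convex collision is left disconnected.
; Cube-face detection, using angles between a Sphere component's offset and the actor's axes, only prints debug output and does not affect gravity.
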(event `self.ReceiveTick`
  (params (DeltaSeconds :type "Float (single-precision)"))
  (`self.ComputeGravityCube` (`SceneComponent.K2_GetComponentLocation` (`self.Sphere`)))
  (for _array_element (`self.GetOverlappingActors` "/Game/ThirdPerson/Blueprints/BP_ThirdPersonCharacter.BP_ThirdPersonCharacter_C")
    (bind _asbp_third_person_character (cast `/Game/ThirdPerson/Blueprints/BP_ThirdPersonCharacter` _array_element))
    (`CharacterMovementComponent.SetGravityDirection` (`Character.CharacterMovement` _asbp_third_person_character) (`KismetMathLibrary.GetDirectionUnitVector` (`self.K2_GetActorLocation` _asbp_third_person_character) (`self.K2_GetActorLocation`)))
    (`KismetSystemLibrary.PrintString` (`KismetSystemLibrary.GetDisplayName` _array_element) true false (struct :`G` 0.66 :`B` 1.0 :`A` 1.0) (`GameplayStatics.GetWorldDeltaSeconds`))))

(fn `AngleBetweenVectors`
  (params (V1 :type "Vector Structure") (V2 :type "Vector Structure"))
  (returns (Angle :type "Float (double-precision)"))
  (return (`KismetMathLibrary.DegAcos` (`KismetMathLibrary.Dot_VectorVector` V1 V2))))

(fn `ComputeGravityCube`
  (params (Positon :type "Vector Structure"))
  (returns (Gravity :type "Vector Structure"))
  (locals (AngleX :type "Float (double-precision)") (AngleY :type "Float (double-precision)") (AngleZ :type "Float (double-precision)"))
  (bind _returnvalue (`KismetMathLibrary.Normal` (- Positon (`self.K2_GetActorLocation`))))
  (bind _angle (`self.AngleBetweenVectors` _returnvalue (`self.GetActorForwardVector`)))
  (bind _output_get (set `local.AngleX` _angle))
  (bind _angle_2 (`self.AngleBetweenVectors` _returnvalue (`self.GetActorRightVector`)))
  (bind _output_get_2 (set `local.AngleY` _angle_2))
  (bind _angle_3 (`self.AngleBetweenVectors` _returnvalue (`self.GetActorUpVector`)))
  (bind _output_get_3 (set `local.AngleZ` _angle_3))
  (bind (_returnvalue_x _returnvalue_y _returnvalue_z) (`KismetMathLibrary.BreakVector` (`KismetMathLibrary.MakeVector` _output_get _output_get_2 _output_get_3)))
  (bind _returnvalue_2 (`BPFL_ShapeGenerators.checkCubeSideByAngle` _returnvalue_x _returnvalue_y _returnvalue_z))
  (`KismetSystemLibrary.PrintString` (`KismetStringLibrary.Conv_VectorToString` _returnvalue_2) true false (struct :`G` 0.66 :`B` 1.0 :`A` 1.0) (`GameplayStatics.GetWorldDeltaSeconds`)))

(fn `UserConstructionScript`
  (locals (VertexColours :type "Array of LinearColor Structure"))
  (`BPFL_ShapeGenerators.GenerateSphereMesh` (`self.ProceduralMesh`) 100.0 12 12)
  (`PrimitiveComponent.SetMaterial` (`self.ProceduralMesh`) 0 "/Game/Materials/M_PCollision.M_PCollision"))