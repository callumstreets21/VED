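; BP_GravityFieldDisk is a disk-shaped gravity field actor built from a procedural mesh.
; Its construction script generates a beveled disk from radius and segment variables.
; Disconnected graph logic would set each overlapping third-person character's gravity direction via ComputeGravity and draw a debug arrow.
; Tick is empty, so that logic never runs in this Blueprint.
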(event `self.ReceiveTick`
  (params (DeltaSeconds :type "Float (single-precision)")))

(fn `UserConstructionScript`
  (`ProceduralMeshGeneratorUtilsBPLibrary.GenerateBeveledDisk` (`self.proceduralMesh`) (`self.innerRadius`) (`self.outerRadius`) (`self.radialSegments`) (`self.tubularSegmenets`)))