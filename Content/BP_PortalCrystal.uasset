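; BP_PortalCrystal is a touch-triggered crystal that changes the state of matching portals when the third-person character overlaps it.
; Tick counts BlockTime down, and overlaps are ignored until it drops below zero.
; A valid overlap finds every BP_Portal, sets Unlocked to false on those sharing the crystal's UnlockNumber, then destroys the crystal.
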(event `self.ReceiveActorBeginOverlap`
  (params (OtherActor :type "Actor Object Reference"))
  (if (< (`self.BlockTime`) 0.0)
    (cast `/Game/ThirdPerson/Blueprints/BP_ThirdPersonCharacter` OtherActor)
    (bind _outactors (`GameplayStatics.GetAllActorsOfClass` "/Game/ThirdPerson/Blueprints/BP_Portal.BP_Portal_C"))
    (for _array_element _outactors
      (if (== (`/Game/ThirdPerson/Blueprints/BP_Portal.UnlockNumber` _array_element) (`self.UnlockNumber`))
        (set `/Game/ThirdPerson/Blueprints/BP_Portal.Unlocked` false _array_element)))
    (`self.K2_DestroyActor`)))

(event `self.ReceiveTick`
  (params (DeltaSeconds :type "Float (single-precision)"))
  (set `self.BlockTime` (- (`self.BlockTime`) DeltaSeconds)))

(fn `UserConstructionScript`)