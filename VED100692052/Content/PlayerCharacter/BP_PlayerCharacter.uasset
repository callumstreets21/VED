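; BP_PlayerCharacter is the player-controlled character, handling movement, camera look and jumping through Enhanced Input.
; On BeginPlay it adds the IM_PlayerMapping context to the owning player controller's input subsystem.
; IA_Move drives movement along the actor's right and forward vectors and maintains a Moving flag.
; IA_Camera feeds controller yaw and pitch, and IA_Jump triggers the built-in character jump.
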(event `self.ReceiveBeginPlay`
  (bind _asplayer_controller (cast `PlayerController` (`self.GetController`)))
  (message `EnhancedInputSubsystemInterface.AddMappingContext` (pcsubsystem `EnhancedInputLocalPlayerSubsystem` _asplayer_controller) "/Game/input/IM_PlayerMapping.IM_PlayerMapping" 0 (struct)))

(event `EnhancedInput|/Game/input/IA/IA_Move`
  (params (ActionValue :type "Vector2D Structure") (ElapsedSeconds :type "Float (double-precision)") (TriggeredSeconds :type "Float (double-precision)") (InputAction :type "InputAction Object Reference" :default "/Game/input/IA/IA_Move.IA_Move"))
  (:`Triggered`
    (`self.AddMovementInput` (`self.GetActorRightVector`) ActionValue_X)
    (`self.AddMovementInput` (`self.GetActorForwardVector`) ActionValue_Y)
    (set `self.Moving` true))
  (:`Completed`
    (set `self.Moving` false)))

(event `EnhancedInput|/Game/input/IA/IA_Camera`
  (params (ActionValue :type "Vector2D Structure") (ElapsedSeconds :type "Float (double-precision)") (TriggeredSeconds :type "Float (double-precision)") (InputAction :type "InputAction Object Reference" :default "/Game/input/IA/IA_Camera.IA_Camera"))
  (:`Triggered`
    (`self.AddControllerYawInput` ActionValue_X)
    (`self.AddControllerPitchInput` ActionValue_Y)))

(event `EnhancedInput|/Game/input/IA/IA_Jump`
  (params (ActionValue :type Boolean) (ElapsedSeconds :type "Float (double-precision)") (TriggeredSeconds :type "Float (double-precision)") (InputAction :type "InputAction Object Reference" :default "/Game/input/IA/IA_Jump.IA_Jump"))
  (:`Triggered`
    (`self.Jump`)))

(fn `UserConstructionScript`)